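; Base chamber Blueprint for NeuroShift that tracks player performance and reports it to the session history.
; RecordHit increments the hit count but zeroes total reaction time, and RecordMistake sets the mistake count to 1 rather than incrementing.
; FinishChamber appends name, accuracy, mistakes and score (the hit count) to BP_NSGameInstance's SessionHistory.
; A debug print and delayed counter reset exist but are disconnected, so counters never reset here.
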(event `RecordHit`
  (params (ReactionTime :type "Float (double-precision)"))
  (set `self.HitCount` (+ (`self.HitCount`) 1))
  (set `self.TotalReactionTime` 0.0))

(event `RecordMistake`
  (bind _output_get (set `self.MistakeCount` 1)))

(event `FinishChamber`
  (bind _asbp_nsgame_instance (cast `/Game/NeuroShift/Blueprints/Core/BP_NSGameInstance` (`GameplayStatics.GetGameInstance`)))
  (`KismetArrayLibrary.Array_Add` (`/Game/NeuroShift/Blueprints/Core/BP_NSGameInstance.SessionHistory` _asbp_nsgame_instance) (make `/Game/NeuroShift/Blueprints/Struct_ChamberResult` (`self.ChamberName`) (/ (`KismetMathLibrary.Conv_IntToDouble` (`self.HitCount`)) (`KismetMathLibrary.Conv_IntToDouble` (+ (`self.HitCount`) (`self.MistakeCount`)))) (`self.MistakeCount`) 0.0 (`self.HitCount`))))

(fn `UserConstructionScript`)