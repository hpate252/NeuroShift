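; BP_Chamber_01 is a chamber Blueprint that turns trigger-zone overlaps into hit, mistake and completion events.
; The green hit zone records a hit with a fixed zero value, the red zone records a mistake, and the finish-door zone finishes the chamber.
; The overlap handlers do not filter the overlapping actor, and BeginPlay, Tick and the construction script add no logic of their own.
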(event `On Component Begin Overlap (FinishZone_Door)`
  (params (OverlappedComponent :type "PrimitiveComponent Object Reference") (OtherActor :type "Actor Object Reference") (OtherComp :type "PrimitiveComponent Object Reference") (OtherBodyIndex :type Integer) (bFromSweep :type Boolean) (SweepResult :type "HitResult Structure (by ref)"))
  (`self.FinishChamber`))

(event `On Component Begin Overlap (MistakeZone_Red)`
  (params (OverlappedComponent :type "PrimitiveComponent Object Reference") (OtherActor :type "Actor Object Reference") (OtherComp :type "PrimitiveComponent Object Reference") (OtherBodyIndex :type Integer) (bFromSweep :type Boolean) (SweepResult :type "HitResult Structure (by ref)"))
  (`self.RecordMistake`))

(event `self.HitZone_Green.OnComponentBeginOverlap`
  (params (OverlappedComponent :type "PrimitiveComponent Object Reference") (OtherActor :type "Actor Object Reference") (OtherComp :type "PrimitiveComponent Object Reference") (OtherBodyIndex :type Integer) (bFromSweep :type Boolean) (SweepResult :type "HitResult Structure (by ref)"))
  (`self.RecordHit` 0.0))

(fn `UserConstructionScript`
  (`parent.UserConstructionScript`))