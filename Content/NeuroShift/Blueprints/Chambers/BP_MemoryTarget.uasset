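; BP_MemoryTarget is a target actor for the memory chamber that can briefly flash a point light.
; ActivateGlow shows the light, waits half a second, then hides it.
; On overlap it looks up BP_MemoryChamber and calls the parent handler, but the CheckPlayerGuess call that would report this target to the chamber is not connected, so it never runs.
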(event `ActivateGlow`
  (`SceneComponent.SetVisibility` (`self.PointLight`) true false)
  (`KismetSystemLibrary.Delay` 0.5)
  (`SceneComponent.SetVisibility` (`self.PointLight`) false false))

(event `self.ReceiveActorBeginOverlap`
  (params (OtherActor :type "Actor Object Reference"))
  (bind _returnvalue (`GameplayStatics.GetActorOfClass` "/Game/NeuroShift/Blueprints/Chambers/BP_MemoryChamber.BP_MemoryChamber_C"))
  (`parent.ReceiveActorBeginOverlap` OtherActor))

(fn `UserConstructionScript`
  (`parent.UserConstructionScript`))