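; BP_MemoryChamber is a Simon-style memory game that plays a sequence of BP_MemoryTarget actors, then checks player guesses.
; FlashNextTarget recursively steps through TargetSequence on one-second delays before enabling the player's turn.
; CheckPlayerGuess advances or resets progress, glowing correct targets and printing results.
; It is unfinished: sequence shuffling and filling, playback start, playback glow and level advancement are disconnected, and BeginPlay only gathers targets.
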(event `CheckPlayerGuess`
  (params (GuessedTarget :type "/Game/NeuroShift/Blueprints/Chambers/BP_MemoryTarget Object Reference"))
  (bind _currentstepindex (`self.CurrentStepIndex`))
  (if (`self.bIsPlayersTurn`)
    (if (== (`|GetArrayItem` (`self.TargetSequence`) _currentstepindex) GuessedTarget)
      (`/Engine/EditorBlueprintResources/StandardMacros.IncrementInt` _currentstepindex
        (:`  `
          (if (> (`self.CurrentStepIndex`) (`self.CurrentLevel`))
            (`KismetSystemLibrary.PrintString` "Round Complete! You Win! ")
            (else
              (`/Game/NeuroShift/Blueprints/Chambers/BP_MemoryTarget.ActivateGlow` GuessedTarget)))))
      (else
        (`KismetSystemLibrary.PrintString` "Wrong")
        (set `self.CurrentStepIndex` 0)))))

(event `self.ReceiveBeginPlay`
  (bind _outactors (`GameplayStatics.GetAllActorsOfClass` "/Game/NeuroShift/Blueprints/Chambers/BP_MemoryTarget.BP_MemoryTarget_C")))

(event `FlashNextTarget`
  (bind _playbackindex (`self.PlaybackIndex`))
  (if (<= _playbackindex (`self.CurrentLevel`))
    (bind _asbp_memory_target (cast `/Game/NeuroShift/Blueprints/Chambers/BP_MemoryTarget` (`|GetArrayItem` (`self.TargetSequence`) _playbackindex)))
    (`KismetSystemLibrary.Delay` 1.0)
    (`/Engine/EditorBlueprintResources/StandardMacros.IncrementInt` _playbackindex
      (:`  `
        (`self.FlashNextTarget`)))
    (else
      (`KismetSystemLibrary.PrintString` "Your Turn!" true true (struct :`R` 0.005208 :`G` 1.0 :`B` 0.04461 :`A` 1.0))
      (set `self.bIsPlayersTurn` true))))

(event `StartFlashingSequence`
  (set `self.bIsPlayersTurn` false)
  (set `self.PlaybackIndex` 0)
  (`self.FlashNextTarget`))

(fn `UserConstructionScript`
  (`parent.UserConstructionScript`))